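; Ghost spawner that places BP_ghost actors at random points inside its Box component bounds.
; BeginPlay spawns an initial batch without counting it and calls the spawn routine on each iteration.
; That routine runs randomly sized waves through a Delay-driven loop, spawning only while the count is below NombreMaxGhosts, then re-triggers itself after a random pause.
; Ghosts_destroy decrements the count to free slots.
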(event `self.ReceiveBeginPlay`
  (bind (_origin _boxextent) (`KismetSystemLibrary.GetComponentBounds` (`self.Box`)))
  (for _ (range 11)
    (`|SpawnActorFromClass` "/Game/Blueprints/BP_ghost.BP_ghost_C" (`KismetMathLibrary.MakeTransform` (`KismetMathLibrary.RandomPointInBoundingBox` _origin _boxextent) (struct) (`self.Scaale_ghosts`)) "AdjustIfPossibleButAlwaysSpawn" "OverrideRootScale" null null)
    (`self.Spawn_ghost`)))

(event `Ghosts_destroy`
  (set `self.Current_nombre_ghosts` (- (`self.Current_nombre_ghosts`) 1)))

(event `Spawn_ghost`
  (bind _variable (`|TemporaryVariable`))
  (bind (_origin _boxextent) (`KismetSystemLibrary.GetComponentBounds` (`self.Box`)))
  (`|AssignmentStatement` _variable)
  (if (<= _variable (`KismetMathLibrary.RandomIntegerInRange` 10 25)) :!label _label
    (`|ExecutionSequence`
      (:`then_0`
        (if (not (>= (`self.Current_nombre_ghosts`) (`self.Nombre_max_ghosts`)))
          (`|SpawnActorFromClass` "/Game/Blueprints/BP_ghost.BP_ghost_C" (`KismetMathLibrary.MakeTransform` (`KismetMathLibrary.RandomPointInBoundingBox` _origin _boxextent) (struct) (`self.Scaale_ghosts`)) "AdjustIfPossibleButAlwaysSpawn" "OverrideRootScale" null null)
          (`/Engine/EditorBlueprintResources/StandardMacros.IncrementInt` (`self.Current_nombre_ghosts`))))
      (:`then_1`
        (`KismetSystemLibrary.Delay` (`KismetMathLibrary.RandomFloatInRange` 0.075 1.0))
        (`|AssignmentStatement` _variable (+ _variable 1))
        (goto _label)))
    (else
      (`KismetSystemLibrary.Delay` (`KismetMathLibrary.RandomFloatInRange` 0.1 1.5))
      (`self.Spawn_ghost`))))

(fn `UserConstructionScript`)