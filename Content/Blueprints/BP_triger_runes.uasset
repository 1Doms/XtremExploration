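; BP_triger_runes is a box trigger that starts a cinematic explosion sequence which kills all ghosts when a Player-tagged actor enters.
; It switches the music manager to cinematic mode, plays the referenced sequence and a big sound.
; After timed delays, it spawns a Niagara explosion at BP_spawn_big_explosion and calls Kill on every BP_ghost.
; It later stops cinematic music and resets its DoOnce, allowing retriggering.
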(event `self.Box.OnComponentBeginOverlap`
  (params (OverlappedComponent :type "PrimitiveComponent Object Reference") (OtherActor :type "Actor Object Reference") (OtherComp :type "PrimitiveComponent Object Reference") (OtherBodyIndex :type Integer) (bFromSweep :type Boolean) (SweepResult :type "HitResult Structure (by ref)"))
  (if (`self.ActorHasTag` OtherActor "Player")
    (`/Engine/EditorBlueprintResources/StandardMacros.DoOnce` false :!label _label
      (:`Completed`
        (bind _returnvalue (`GameplayStatics.GetActorOfClass` "/Game/Blueprints/BP_music_manager.BP_music_manager_C"))
        (`/Game/Blueprints/BP_music_manager.Cinematic` _returnvalue)
        (`MovieSceneSequencePlayer.Play` (`LevelSequenceActor.SequencePlayer` (`self.Cinematic_ref`)))
        (`GameplayStatics.PlaySound2D` "/Game/Assets/Sounds/big_sfx_Cue.big_sfx_Cue" 1.0 1.0 0.0 null null)
        (bind _returnvalue_2 (`GameplayStatics.GetActorOfClass` "/Game/Blueprints/BP_spawn_big_explosion.BP_spawn_big_explosion_C"))
        (`KismetSystemLibrary.Delay` 5.0)
        (`NiagaraFunctionLibrary.SpawnSystemAtLocation` "/Game/Assets/Effects/Niagara/NS_big_explosion.NS_big_explosion" (`self.K2_GetActorLocation` _returnvalue_2))
        (`KismetSystemLibrary.Delay` 0.15)
        (bind _outactors (`GameplayStatics.GetAllActorsOfClass` "/Game/Blueprints/BP_ghost.BP_ghost_C"))
        (for _array_element _outactors
          (bind _asbp_ghost (cast `/Game/Blueprints/BP_ghost` _array_element))
          (`/Game/Blueprints/BP_ghost.Kill` _asbp_ghost))
        (`KismetSystemLibrary.Delay` 10.0)
        (bind _returnvalue_3 (`GameplayStatics.GetActorOfClass` "/Game/Blueprints/BP_music_manager.BP_music_manager_C"))
        (`/Game/Blueprints/BP_music_manager.Stop_cinematic` _returnvalue_3)
        (`KismetSystemLibrary.Delay` 5.0)
        (goto _label :!via `Reset`)))))

(fn `UserConstructionScript`)