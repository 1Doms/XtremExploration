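; Music manager that runs the game's background music and switches audio between normal, swimming and cinematic states.
; BeginPlay starts a creepy track and an underwater ambience, with the sea sound class muted.
; Swim events use SM_main class overrides to lower and pitch down main audio, raise the sea layer, then revert, playing a splash at the player.
; Cinematic events swap music for a joyful track, stopping it after a short delay.
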(event `self.ReceiveBeginPlay`
  (`GameplayStatics.SpawnSound2D` "/Game/Assets/Sounds/Creepy_music_1_Cue.Creepy_music_1_Cue" 1.0 1.0 0.0 null false false)
  (`GameplayStatics.SpawnSound2D` "/Game/Assets/Sounds/Deep_Sea_Dive_Sound_Effect_Cue.Deep_Sea_Dive_Sound_Effect_Cue" 1.0 1.0 0.0 null false false)
  (`GameplayStatics.SetSoundMixClassOverride` "/Game/Assets/Sounds/SM_main.SM_main" "/Game/Assets/Sounds/SC_sea.SC_sea" 0.0 1.0 0.2)
  (`GameplayStatics.PushSoundMixModifier` "/Game/Assets/Sounds/SM_main.SM_main"))

(event `Swiming`
  (`GameplayStatics.SetSoundMixClassOverride` "/Game/Assets/Sounds/SM_main.SM_main" "/Game/Assets/Sounds/SC_main.SC_main" 0.75 0.5 0.2)
  (`GameplayStatics.PushSoundMixModifier` "/Game/Assets/Sounds/SM_main.SM_main")
  (`GameplayStatics.SetSoundMixClassOverride` "/Game/Assets/Sounds/SM_main.SM_main" "/Game/Assets/Sounds/SC_sea.SC_sea" 1.0 1.0 0.2)
  (`GameplayStatics.PushSoundMixModifier` "/Game/Assets/Sounds/SM_main.SM_main")
  (`GameplayStatics.PlaySoundAtLocation` "/Game/Assets/Sounds/Water_jumping_sound_effects_Cue.Water_jumping_sound_effects_Cue" (`self.K2_GetActorLocation` (`GameplayStatics.GetPlayerCharacter` 0)) (struct) 1.0 1.0 0.0 "/Game/Assets/Sounds/SA_wetr_dive.SA_wetr_dive" null null null))

(event `Stop_swiming`
  (`GameplayStatics.SetSoundMixClassOverride` "/Game/Assets/Sounds/SM_main.SM_main" "/Game/Assets/Sounds/SC_main.SC_main" 1.0 1.0 0.2)
  (`GameplayStatics.PushSoundMixModifier` "/Game/Assets/Sounds/SM_main.SM_main")
  (`GameplayStatics.SetSoundMixClassOverride` "/Game/Assets/Sounds/SM_main.SM_main" "/Game/Assets/Sounds/SC_sea.SC_sea" 0.0 1.0 0.2)
  (`GameplayStatics.PushSoundMixModifier` "/Game/Assets/Sounds/SM_main.SM_main")
  (`GameplayStatics.PlaySoundAtLocation` "/Game/Assets/Sounds/Water_jumping_sound_effects_Cue.Water_jumping_sound_effects_Cue" (`self.K2_GetActorLocation` (`GameplayStatics.GetPlayerCharacter` 0)) (struct) 1.0 1.0 0.0 "/Game/Assets/Sounds/SA_wetr_dive.SA_wetr_dive" null null null))

(event `Cinematic`
  (bind _returnvalue (`GameplayStatics.CreateSound2D` "/Game/Assets/Sounds/Music_joyeuse_Cue.Music_joyeuse_Cue" 1.0 1.0 0.0 null))
  (`AudioComponent.Play` _returnvalue 0.0)
  (`GameplayStatics.SetSoundMixClassOverride` "/Game/Assets/Sounds/SM_main.SM_main" "/Game/Assets/Sounds/SC_music.SC_music" 0.0 1.0 0.5)
  (`GameplayStatics.SetSoundMixClassOverride` "/Game/Assets/Sounds/SM_main.SM_main" "/Game/Assets/Sounds/SC_music_cinematic.SC_music_cinematic" 1.0 1.0 0.5)
  (`GameplayStatics.PushSoundMixModifier` "/Game/Assets/Sounds/SM_main.SM_main"))

(event `Stop_cinematic`
  (`GameplayStatics.SetSoundMixClassOverride` "/Game/Assets/Sounds/SM_main.SM_main" "/Game/Assets/Sounds/SC_music_cinematic.SC_music_cinematic" 0.0)
  (`GameplayStatics.SetSoundMixClassOverride` "/Game/Assets/Sounds/SM_main.SM_main" "/Game/Assets/Sounds/SC_music.SC_music")
  (`GameplayStatics.PushSoundMixModifier` "/Game/Assets/Sounds/SM_main.SM_main")
  (`KismetSystemLibrary.Delay` 1.25)
  (`AudioComponent.Stop` (stale `Cinematic` _returnvalue))
  (`GameplayStatics.SetSoundMixClassOverride` "/Game/Assets/Sounds/SM_main.SM_main" "/Game/Assets/Sounds/SC_music_cinematic.SC_music_cinematic")
  (`GameplayStatics.PushSoundMixModifier` "/Game/Assets/Sounds/SM_main.SM_main"))

(fn `UserConstructionScript`)