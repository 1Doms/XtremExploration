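; BP_water_triger is a water volume that switches BP_CustomTPS characters into and out of swimming, with an optional current.
; Its box overlaps react only to actors tagged "Water", calling Swiming on entry and StopSwiming on exit.
; With Courant enabled, a very fast looping timer adds velocity along the Arrow's forward vector while InCourant is true.
; Exit clears that flag, re-sets rather than clears the timer, and subtracts one push.
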(event `self.Box.OnComponentBeginOverlap`
  (params (OverlappedComponent :type "PrimitiveComponent Object Reference") (OtherActor :type "Actor Object Reference") (OtherComp :type "PrimitiveComponent Object Reference") (OtherBodyIndex :type Integer) (bFromSweep :type Boolean) (SweepResult :type "HitResult Structure (by ref)"))
  (if (`self.ActorHasTag` OtherActor "Water")
    (bind _asbp_custom_tps (cast `/Game/Blueprints/BP_CustomTPS` OtherActor))
    (`/Game/Blueprints/BP_CustomTPS.Swiming` _asbp_custom_tps)
    (if (`self.Courant?`)
      (set `self.In_courant` true)
      (`KismetSystemLibrary.K2_SetTimerDelegate` (delegate `Courant`) 0.001 true :!label _label))))

(event `Courant`
  (if (`self.In_courant`)
    (bind _charactermovement (`Character.CharacterMovement` (stale `self.Box.OnComponentBeginOverlap` _asbp_custom_tps)))
    (set `MovementComponent.Velocity` (+ (* (`SceneComponent.GetForwardVector` (`self.Arrow`)) (`self.Courant_power`)) (`MovementComponent.Velocity` _charactermovement)) _charactermovement)))

(event `self.Box.OnComponentEndOverlap`
  (params (OverlappedComponent :type "PrimitiveComponent Object Reference") (OtherActor :type "Actor Object Reference") (OtherComp :type "PrimitiveComponent Object Reference") (OtherBodyIndex :type Integer))
  (if (`self.ActorHasTag` OtherActor "Water")
    (bind _asbp_custom_tps (cast `/Game/Blueprints/BP_CustomTPS` OtherActor))
    (`/Game/Blueprints/BP_CustomTPS.Stop_swiming` _asbp_custom_tps)
    (if (`self.Courant?`)
      (set `self.In_courant` false)
      (`|ExecutionSequence`
        (:`then_0`
          (goto _label))
        (:`then_1`
          (bind _charactermovement (`Character.CharacterMovement` _asbp_custom_tps))
          (set `MovementComponent.Velocity` (- (`MovementComponent.Velocity` _charactermovement) (* (`SceneComponent.GetForwardVector` (`self.Arrow`)) (`self.Courant_power`))) _charactermovement))))))

(fn `UserConstructionScript`)