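; Ghost character that wanders, always faces the player and dies when rammed at high speed.
; Self-recalling delayed events set random velocities and play haunting sounds at random intervals.
; A fast player hit shares the Kill path, which spawns effects and sound, calls GhostsDestroy on BP_spawn_ghosts and destroys the actor.
; Slower player hits only show a block effect aligned to the hit normal, throttled by a DoOnce with delayed reset.
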(event `Kill`
  (`NiagaraFunctionLibrary.SpawnSystemAtLocation` "/Game/Assets/Effects/Niagara/NS_ghost_kill.NS_ghost_kill" (`self.K2_GetActorLocation`) (struct) (`self.Sclae_system`) :!label _label)
  (bind _returnvalue (`GameplayStatics.GetActorOfClass` "/Game/Blueprints/BP_spawn_ghosts.BP_spawn_ghosts_C"))
  (`/Game/Blueprints/BP_spawn_ghosts.Ghosts_destroy` _returnvalue)
  (`GameplayStatics.PlaySoundAtLocation` "/Game/Assets/Sounds/Impact_sound_1_Cue.Impact_sound_1_Cue" (`self.K2_GetActorLocation`) (struct) 2.5 1.0 0.0 "/Game/Assets/Sounds/SA_ghost_scream.SA_ghost_scream" null null null)
  (`self.K2_DestroyActor`))

(event `self.ReceiveHit`
  (params (MyComp :type "PrimitiveComponent Object Reference") (Other :type "Actor Object Reference") (OtherComp :type "PrimitiveComponent Object Reference") (bSelfMoved :type Boolean) (HitLocation :type "Vector Structure") (HitNormal :type "Vector Structure") (NormalImpulse :type "Vector Structure") (Hit :type "HitResult Structure (by ref)"))
  (bind (_returnvalue_roll _returnvalue_pitch _returnvalue_yaw) (`KismetMathLibrary.BreakRotator` (`KismetMathLibrary.Conv_VectorToRotator` HitNormal)))
  (if (`self.ActorHasTag` Other "Player")
    (bind _ascharacter (cast `Character` Other))
    (if (>= (`KismetMathLibrary.VSize` (`MovementComponent.Velocity` (`Character.CharacterMovement` _ascharacter))) 1500.0)
      (goto _label)
      (else
        (`/Engine/EditorBlueprintResources/StandardMacros.DoOnce` false :!label _label_2
          (:`Completed`
            (`NiagaraFunctionLibrary.SpawnSystemAtLocation` "/Game/Assets/Effects/Niagara/NS_block.NS_block" HitLocation (`KismetMathLibrary.MakeRotator` (+ _returnvalue_roll 90.0) (+ _returnvalue_pitch 90.0) (+ _returnvalue_yaw 90.0)) (2.0 2.0 2.0))
            (`KismetSystemLibrary.Delay` 1.15)
            (goto _label_2 :!via `Reset`)))))))

(event `self.ReceiveBeginPlay`
  (`self.Move`)
  (`self.Sound`))

(event `self.ReceiveTick`
  (params (DeltaSeconds :type "Float (single-precision)"))
  (`self.K2_SetActorRotation` (`KismetMathLibrary.FindLookAtRotation` (`self.K2_GetActorLocation`) (`self.K2_GetActorLocation` (`GameplayStatics.GetPlayerCharacter` 0)))))

(event `Move`
  (set `MovementComponent.Velocity` (* (`KismetMathLibrary.MakeVector` (`KismetMathLibrary.RandomFloatInRange` -1.0 1.0) (`KismetMathLibrary.RandomFloatInRange` -1.0 1.0) (`KismetMathLibrary.RandomFloatInRange` -1.0 1.0)) (`self.Movement_speed`)) (`self.CharacterMovement`))
  (`KismetSystemLibrary.Delay` (`KismetMathLibrary.RandomFloatInRange` 0.1 10.0))
  (`self.Move`))

(event `Sound`
  (bind _returnvalue (`self.K2_GetActorLocation`))
  (`GameplayStatics.PlaySoundAtLocation` "/Game/Assets/Sounds/Female_Ghost_Sound_Effect_Cue.Female_Ghost_Sound_Effect_Cue" _returnvalue (struct) 0.5 1.0 0.0 "/Game/Assets/Sounds/SA_ghost_scream.SA_ghost_scream" null null null)
  (`GameplayStatics.PlaySoundAtLocation` "/Game/Assets/Sounds/Wendigo_Sounds_1_Cue.Wendigo_Sounds_1_Cue" _returnvalue (struct) 0.5 1.0 0.0 "/Game/Assets/Sounds/SA_ghost_scream.SA_ghost_scream" null null null)
  (`KismetSystemLibrary.Delay` (`KismetMathLibrary.RandomFloatInRange` 0.5 5.0))
  (`self.Sound`))

(fn `UserConstructionScript`)